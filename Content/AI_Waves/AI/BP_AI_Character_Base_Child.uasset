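; BP_AI_Character_Base_Child is an AI wave character, derived from BP_AI_Character_Base, that attacks on contact.
; Any capsule overlap, with no filter on the other actor, plays the MagnitexAttack animation directly on the mesh and immediately applies radial damage around itself.
; The damage ignore list holds only child actors of the first AI target, not the target or this character.
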(event OnComponentBeginOverlap(CapsuleComponent)
  (params (OverlappedComponent :type Primitive%20Component%20Object%20Reference) (OtherActor :type Actor%20Object%20Reference) (OtherComp :type Primitive%20Component%20Object%20Reference) (OtherBodyIndex :type Integer) (bFromSweep :type Boolean) (SweepResult :type Hit%20Result%20Structure%20%28by%20ref%29))
  (Components|Animation|PlayAnimation (Variables|Character|GetMesh) "/Game/Content/Characters/Dreamon3Magnitex/MagnitexAttack.MagnitexAttack" false)
  (Game|Damage|ApplyRadialDamage 5e+01 (Transformation|GetActorLocation) 1e+02 0 (Actor|GetAllChildActors (CallFunction|GetFirstAITargetActor "/Game/AI_Waves/AI/BP_AI_Character_Base.BP_AI_Character_Base_C") true) self 0 false "ECC_Visibility"))

(event EventBeginPlay
  (|CallParentFunction) ; This node is disabled and will not be called.\nDrag off pins to build functionality.
)

(event Collision|EventActorBeginOverlap
  (params (OtherActor :type Actor%20Object%20Reference)))

(event EventTick
  (params (DeltaSeconds :type Float%20%28single-precision%29)))

(fn ConstructionScript
  (|CallParentFunction))