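; BP_A_Waypoint is an AI waypoint actor that links to other actors through its AITarget array.
; GetNextTargetActor picks a random entry with a HasTarget flag, but rerolls between validity check and return, so the two may differ.
; The construction script resets ShowDebugTargets, flushes persistent debug lines, draws timed arrows to valid targets and labels the waypoint with its name.
; The event graph holds no logic.
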(event EventBeginPlay)

(event Collision|EventActorBeginOverlap
  (params (OtherActor :type Actor%20Object%20Reference)))

(event EventTick
  (params (DeltaSeconds :type Float%20%28single-precision%29)))

(fn ConstructionScript
  ;[1 1 1] Draw lines to my AI Targets
  (Variables|Default|SetshowDebugTargets false)
  (Rendering|Debug|FlushPersistentDebugLines)
  (for _array_element (Variables|Default|GetAI_Target)
    (Utilities|IsValid _array_element
      (:Is%20Valid
        (Rendering|Debug|DrawDebugArrow (Transformation|GetActorLocation) (Transformation|GetActorLocation _array_element) 1e+01 "(R=0.000000,G=0.432292,B=0.000000,A=1.000000)" 3e+01 3.0))))
  ;[1 1 1] Add some text with my name
  (Rendering|Components|TextRender|SetText (Variables|Default|GetTextRender) (Utilities|Text|ToText(String) (Utilities|GetDisplayName self))))

(fn GetNextTargetActor
  (bind _ai_target (Variables|Default|GetAI_Target))
  (bind _returnvalue (Utilities|Array|LastIndex _ai_target))
  (bind _returnvalue_2 (Math|Random|RandomIntegerinRange 0 _returnvalue))
  (bind _output (Utilities|Array|Get(acopy) _ai_target _returnvalue_2))
  (Utilities|IsValid _output
    (:Is%20Valid
      (return _output true))
    (:Is%20Not%20Valid
      (return 0 false))))