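; Base enemy AI character for a wave game that randomly targets either the player or a non-AI target actor on spawn.
; MoveToTarget uses continuously tracked AI moves, re-issued after a delay, while non-attackers follow interface waypoints until a gate locks in the final target.
; Damage redirects it to the player, and death increments Teddy's DeathCounter.
; Player capsule contact triggers attack animation and radial damage; leaving the sphere redirects it to the non-AI target.
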(event OnComponentBeginOverlap(CapsuleComponent)
  (params (OverlappedComponent :type Primitive%20Component%20Object%20Reference) (OtherActor :type Actor%20Object%20Reference) (OtherComp :type Primitive%20Component%20Object%20Reference) (OtherBodyIndex :type Integer) (bFromSweep :type Boolean) (SweepResult :type Hit%20Result%20Structure%20%28by%20ref%29))
  (Utilities|Casting|CastToTeddyCharacter OtherActor)
  (Components|Animation|PlayAnimation (Variables|Character|GetMesh) "/Game/Content/Characters/Dreamon3Magnitex/MagnitexAttack.MagnitexAttack" true)
  (Game|Damage|ApplyRadialDamage 5e+01 (Transformation|GetActorLocation) 1e+02 0 (Actor|GetAllChildActors (CallFunction|GetFirstAITargetActor "BP_AI_Character_Base_C") true) self 0 false "ECC_Visibility"))

(event OnComponentEndOverlap(Sphere)
  (params (OverlappedComponent :type Primitive%20Component%20Object%20Reference) (OtherActor :type Actor%20Object%20Reference) (OtherComp :type Primitive%20Component%20Object%20Reference) (OtherBodyIndex :type Integer))
  (Utilities|Casting|CastToTeddyCharacter OtherActor)
  (CallFunction|MovetoTarget (CallFunction|GetFirstAITargetActor "/Game/AI_Waves/AI/BP_NonAITarget_Actor.BP_NonAITarget_Actor_C")))

(event Custom|AIWaypointReached
  (params (waypoint :type Actor%20Object%20Reference))
  ;[1 1 1] If overlapping an AI Waypoint, ask for a new waypoint. (If attacking player ignore. If there are no more waypoints - ie empty array - then go for tor the finallTargetActor and ignore any subsequent waypoints)
  (if (not (Variables|Default|GetAttackPlayer)) ; ignore waypoints if attacking player
    (Utilities|FlowControl|Gate false :!label _label
      (:Exit
        (if (Utilities|DoesObjectImplementInterface waypoint "/Game/AI_Waves/AI/BPI_AI_Waypoint.BPI_AI_Waypoint_C")
          (bind (_actorref _hastarget) (Class|BPIAIWaypoint|GetNextTargetActor(Message) waypoint))
          (if _hastarget
            (CallFunction|MovetoTarget _actorref) ; Move to waypoint next actor
            (else
              (CallFunction|MovetoTarget (Variables|Default|GetfinalTargetActor)) ; move to the final target (close the gate to ignore other waypoints)
              (goto _label Close))))))))

(event Custom|init
  ;[1 1 1] Decide which actor is our target
  (Utilities|Casting|CastToGM_BasicAIWaves (Game|GetGameMode)) ; hard-coded to game mode - ideally use a Game mode 'interface' instead
  (Variables|Default|SetAttackPlayer (Math|Random|RandomBool))
  (CallFunction|MovetoTarget (select (Variables|Default|GetAttackPlayer) (Game|GetPlayerCharacter 0) (CallFunction|GetFirstAITargetActor "/Game/AI_Waves/AI/BP_NonAITarget_Actor.BP_NonAITarget_Actor_C")))
  (Variables|Default|SetfinalTargetActor (select (Variables|Default|GetAttackPlayer) (Game|GetPlayerCharacter 0) (CallFunction|GetFirstAITargetActor "/Game/AI_Waves/AI/BP_NonAITarget_Actor.BP_NonAITarget_Actor_C"))))

(event Custom|MoveToTarget
  (params (AITargetActor :type Actor%20Object%20Reference))
  ;[1 1 1] Start AI using Blueprint Method
  (AI|AIMoveTo (AI|GetAIController self) "0, 0, 0" AITargetActor -1.0 "Enable" "Enable" true true true ; using 'continuos' tracking - they never stop!
    (:OnRequestFailed
      _)
    (:OnMoveFinished
      _))
  ;[1 1 1] Try looking again for the AI Target if we lose it
  (Utilities|FlowControl|Delay 0.5) ; wait a moment
  (CallFunction|MovetoTarget AITargetActor))

(event Collision|EventActorBeginOverlap
  (params (OtherActor :type Actor%20Object%20Reference))
  ;[1 1 1] Overlap Event
  (Utilities|FlowControl|Sequence
    (:then_0
      (CallFunction|AIWaypointReached OtherActor))
    (:then_1)))

(event EventBeginPlay
  (Variables|Default|SetEnemyHealth (Variables|Default|GetMaxEnemyHealth))
  (CallFunction|Init)
  (bind _asteddy_character (Utilities|Casting|CastToTeddyCharacter (Game|GetPlayerCharacter 0)))
  (Variables|Default|SetTeddy _asteddy_character))

(event Game|Damage|EventAnyDamage
  (params (Damage :type Float%20%28single-precision%29) (DamageType :type Damage%20Type%20Object%20Reference) (InstigatedBy :type Controller%20Object%20Reference) (DamageCauser :type Actor%20Object%20Reference))
  (bind _teddy (Variables|Default|GetTeddy))
  ;[1 1 1] AI takes damage and dies
  (Variables|Default|SetEnemyHealth (- (Variables|Default|GetEnemyHealth) Damage))
  (Development|PrintString "target damaged")
  (if (<= (Variables|Default|GetEnemyHealth) 0.0)
    (Variables|/Game/Content/Characters/Teddy/TeddyAssets/TeddyCharacter.TeddyCharacter_C|SetDeathCounter _teddy (+ (Variables|/Game/Content/Characters/Teddy/TeddyAssets/TeddyCharacter.TeddyCharacter_C|GetDeathCounter _teddy) 1))
    (Actor|DestroyActor)
    (Development|PrintString "Target is dead" true true "(R=1.000000,G=0.000000,B=0.829394,A=1.000000)")
    (else
      (CallFunction|MovetoTarget (Variables|Default|GetTeddy)))))

(event EventTick
  (params (DeltaSeconds :type Float%20%28single-precision%29)))

(fn ConstructionScript)

(fn GetFirstAITargetActor
  (params (actorClass :type Actor%20Class%20Reference))
  (bind _outactors (Actor|GetAllActorsOfClass actorClass))
  (return (Utilities|Array|Get(acopy) _outactors)))