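; Bug enemy for AI waves that attacks the Teddy player character and otherwise heads for a non-AI target actor.
; Capsule overlap starts a delay-based loop that plays the attack animation and sends damage about once a second while Teddy is alive and in range.
; Leaving the capsule clears range and restores the animation Blueprint.
; Leaving the sphere, or an interrupted attack, sends the bug back toward its target.
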(event OnComponentEndOverlap(Sphere)
  (params (OverlappedComponent :type Primitive%20Component%20Object%20Reference) (OtherActor :type Actor%20Object%20Reference) (OtherComp :type Primitive%20Component%20Object%20Reference) (OtherBodyIndex :type Integer))
  ;[1 0.6458 0] End overlap of sphere != in range, moves to child.
  (Utilities|Casting|CastToTeddyCharacter OtherActor)
  (Variables|Default|SetInRange false)
  (Default|MovetoTarget self (CallFunction|GetFirstAITargetActor "/Game/AI_Waves/AI/BP_NonAITarget_Actor.BP_NonAITarget_Actor_C")))

(event OnComponentBeginOverlap(Capsule)
  (params (OverlappedComponent :type Primitive%20Component%20Object%20Reference) (OtherActor :type Actor%20Object%20Reference) (OtherComp :type Primitive%20Component%20Object%20Reference) (OtherBodyIndex :type Integer) (bFromSweep :type Boolean) (SweepResult :type Hit%20Result%20Structure%20%28by%20ref%29))
  ;[1 0 0.1818] Overlap = in range, end overlap != in range. If in range, attack indefinitely, if not, carry on to child.
  (Utilities|Casting|CastToTeddyCharacter OtherActor)
  (Variables|Default|SetInRange true)
  (CallFunction|Attack))

(event OnComponentEndOverlap(Capsule)
  (params (OverlappedComponent :type Primitive%20Component%20Object%20Reference) (OtherActor :type Actor%20Object%20Reference) (OtherComp :type Primitive%20Component%20Object%20Reference) (OtherBodyIndex :type Integer))
  ;[1 0 0.1818] Overlap = in range, end overlap != in range. If in range, attack indefinitely, if not, carry on to child.
  (Utilities|Casting|CastToTeddyCharacter OtherActor)
  (Variables|Default|SetInRange false)
  (Components|Animation|SetAnimationMode (Variables|Character|GetMesh) "AnimationBlueprint"))

(event Custom|Attack
  (bind _teddy (Variables|Default|GetTeddy))
  ;[1 0 0.1818] Overlap = in range, end overlap != in range. If in range, attack indefinitely, if not, carry on to child.
  (if (Variables|Default|GetInRange) :!label _label
    (Components|Animation|PlayAnimation (Variables|Character|GetMesh) "/Game/Content/Characters/Dreamon1TheBug/CameronBug/ShadowBug_Attack.ShadowBug_Attack" false)
    (Utilities|FlowControl|Delay 0.1)
    (if (not (Variables|/Game/Content/Characters/Teddy/TeddyAssets/TeddyCharacter.TeddyCharacter_C|GetIsDead _teddy))
      (if (Variables|Default|GetInRange)
        (Class|TeddyInterface|InDamage(Message) _teddy (Variables|Default|GetAttackDamage))
        (Utilities|FlowControl|Delay 1.0)
        (goto _label)
        (else
          _)))
    (Components|Animation|SetAnimationMode (Variables|Character|GetMesh) "AnimationBlueprint")
    (CallFunction|MovetoTarget (CallFunction|GetFirstAITargetActor "/Game/AI_Waves/AI/BP_NonAITarget_Actor.BP_NonAITarget_Actor_C"))
    (else
      (Components|Animation|SetAnimationMode (Variables|Character|GetMesh) "AnimationBlueprint"))))

(event EventBeginPlay
  (|CallParentFunction) ; This node is disabled and will not be called.\nDrag off pins to build functionality.
)

(event Collision|EventActorBeginOverlap
  (params (OtherActor :type Actor%20Object%20Reference))
  (|CallParentFunction OtherActor) ; This node is disabled and will not be called.\nDrag off pins to build functionality.
)

(fn ConstructionScript
  (|CallParentFunction))