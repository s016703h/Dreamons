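; Game mode that runs basic AI enemy waves, starting wave 1 on BeginPlay.
; StartWave builds a per-wave actor tag and starts a looping timer that repeatedly spawns Hunch_BP at a random spawn point carrying that tag.
; ResetAndStartNewWave stores an attack-player-on-spawn flag, destroys existing AI characters, clears the timer and starts the requested wave.
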(event EventBeginPlay
  (CallFunction|StartWave 1))

(fn ConstructionScript)

(fn SpawnAI
  ;[1 1 1] Pick a spawn point from the level
  (bind _outactors (Actor|GetAllActorswithTag (Variables|Default|GetWaveSpawnTag)))
  (bind _output_get (LocalVariables|SetLocalVar_spawnpoint (Utilities|Array|Get(acopy) _outactors (Math|Random|RandomIntegerinRange 0 (Utilities|Array|LastIndex _outactors)))))
  (Utilities|IsValid _output_get ; is the spawnpoint valid?
    (:Is%20Valid
      ;[1 1 1] Spawn the AI
      (AI|SpawnAIFromClass "/Game/AI_Waves/AI/Hunch_BP.Hunch_BP_C" 0 (Transformation|GetActorLocation (LocalVariables|GetLocalVar_spawnpoint)) (Transformation|GetActorRotation (LocalVariables|GetLocalVar_spawnpoint)) false))
    (:Is%20Not%20Valid
      ;[1 1 1] no actors with this WaveID were found - check the level has spawn points with the correct ActorTags. eg: 'Spawn_Wave1'
      (Development|PrintString (Utilities|String|Append "No Spawn Point Found for: " (Utilities|String|ToString(Name) (Variables|Default|GetWaveSpawnTag)))))))

(fn StartWave
  (params (waveID :type Integer))
  (bind _output_get (Variables|Default|SetcurrentWaveID waveID)) ; remember our wave ID
  ;[1 1 1] create the relevant actor tag to find the spawn points for this wave
  (Variables|Default|SetWaveSpawnTag (Utilities|String|StringToName (Utilities|String|Append "Spawn_Wave" (Utilities|String|ToString(Integer) _output_get))))
  ;[1 1 1] Setup timer to spawn new AIs
  (bind _returnvalue (Utilities|Time|SetTimerbyFunctionName 0 "spawnAI" 3.0 true))
  (Variables|Default|SetwaveTimer _returnvalue) ; used to cancel or manipulate the timer elsewhere
  (Development|PrintString (Utilities|String|Append "starting wave:  " (Utilities|String|ToString(Integer) (Variables|Default|GetcurrentWaveID)))))

(fn ResetandStartNewWave
  (params (waveID :type Integer) (attackPlayer :type Boolean))
  ;[1 1 1] Desytoy any remaining enemy AI's then start a new wave
  (Variables|Default|SetattackPlayerOnSpawn attackPlayer)
  (bind _outactors (Actor|GetAllActorsOfClass "/Game/AI_Waves/AI/BP_AI_Character_Base.BP_AI_Character_Base_C"))
  (Actor|DestroyActor _outactors)
  (Utilities|Time|ClearandInvalidateTimerbyHandle (Variables|Default|GetwaveTimer))
  (CallFunction|StartWave waveID))